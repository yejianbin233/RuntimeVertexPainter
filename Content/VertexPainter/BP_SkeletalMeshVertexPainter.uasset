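; BP_SkeletalMeshVertexPainter is a test actor that paints skeletal mesh vertices red inside a sphere centred on a movable static mesh.
; Each Tick it gathers override color info for vertices within Radius of that mesh and applies it to LOD 0 of the SkeletalMesh.
; BeginPlay enables player input and halves global time dilation, while the 1 and 2 keys nudge the brush mesh along its relative Y axis.
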(event EventBeginPlay
  (Input|EnableInput self (Game|GetPlayerController 0))
  (Utilities|Time|SetGlobalTimeDilation 0.5))

(event Collision|EventActorBeginOverlap
  (params (OtherActor :type Actor%20Object%20Reference)))

(event EventTick
  (params (DeltaSeconds :type Float%20%28single-precision%29))
  (bind _returnvalue (Class|VertexPainterLibrary|GetSkeletalMeshVertexOverrideColorInfoinSphere (Variables|Default|GetSkeletalMesh) 0 (Transformation|GetWorldLocation (Variables|Default|GetStaticMesh)) (Variables|Default|GetRadius) "(R=1.000000,G=0.000000,B=0.000000,A=1.000000)"))
  (Class|VertexPainterLibrary|OverrideSkeletalMeshVertexColor (Variables|Default|GetSkeletalMesh) 0 _returnvalue))

(event Input|KeyboardEvents|1
  (params (Key :type Key%20Structure :default "None"))
  (:Pressed
    (Transformation|AddRelativeLocation (Variables|Default|GetStaticMesh) (Math|Vector|MakeVector 0.0 1e+01 0.0) false false)))

(event Input|KeyboardEvents|2
  (params (Key :type Key%20Structure :default "None"))
  (:Pressed
    (Transformation|AddRelativeLocation (Variables|Default|GetStaticMesh) (Math|Vector|MakeVector 0.0 -1e+01 0.0) false false)))

(fn ConstructionScript)